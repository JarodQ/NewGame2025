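; Sliding dungeon door that sinks when something overlaps its Trigger and rises again when the overlap ends, with no filter on the overlapping actor.
; Separate open and close timelines, each played from start, lerp the Door component's relative Z toward fixed lowered and raised heights.
; Each update lerps from the current location rather than a stored start, and neither timeline stops the other.
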(event `self.Trigger.OnComponentBeginOverlap`
  (params (OverlappedComponent :type "PrimitiveComponent Object Reference") (OtherActor :type "Actor Object Reference") (OtherComp :type "PrimitiveComponent Object Reference") (OtherBodyIndex :type Integer) (bFromSweep :type Boolean) (SweepResult :type "HitResult Structure (by ref)"))
  (bind _door (`self.Door`))
  (bind (_relativelocation_x _relativelocation_y) (`KismetMathLibrary.BreakVector` (`SceneComponent.RelativeLocation` _door)))
  ;[0.09375 0.09375 0.09375 1 30] Open Door
  (bind (_direction _alpha) (`Timeline|Door Open Anim` :!via `PlayFromStart`)
    (:`Update`
      (bind (_returnvalue_x _returnvalue_y _returnvalue_z) (`KismetMathLibrary.BreakVector` (`KismetMathLibrary.VLerp` (`SceneComponent.RelativeLocation` _door) (`KismetMathLibrary.MakeVector` _relativelocation_x _relativelocation_y -100.0) _alpha)))
      (`SceneComponent.K2_SetRelativeLocation` _door (`KismetMathLibrary.MakeVector` _returnvalue_x _returnvalue_y _returnvalue_z) false false))))

(event `self.Trigger.OnComponentEndOverlap`
  (params (OverlappedComponent :type "PrimitiveComponent Object Reference") (OtherActor :type "Actor Object Reference") (OtherComp :type "PrimitiveComponent Object Reference") (OtherBodyIndex :type Integer))
  (bind _door (`self.Door`))
  (bind (_relativelocation_x _relativelocation_y) (`KismetMathLibrary.BreakVector` (`SceneComponent.RelativeLocation` _door)))
  ;[0.09375 0.09375 0.09375 1 30] Close Door
  (bind (_direction _alpha) (`Timeline|Door Close Anim` :!via `PlayFromStart`)
    (:`Update`
      (bind (_returnvalue_x _returnvalue_y _returnvalue_z) (`KismetMathLibrary.BreakVector` (`KismetMathLibrary.VLerp` (`SceneComponent.RelativeLocation` _door) (`KismetMathLibrary.MakeVector` _relativelocation_x _relativelocation_y 130.0) _alpha)))
      (`SceneComponent.K2_SetRelativeLocation` _door (`KismetMathLibrary.MakeVector` _returnvalue_x _returnvalue_y _returnvalue_z) false false))))

(fn `UserConstructionScript`)