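; BP_Door is an interactable door actor that swings open and closed when Interact is triggered.
; Interact checks IsOpen and calls OpenDoor or CloseDoor, which set the flag and play a sound at the actor's location.
; A single timeline drives the Door component's relative yaw, playing forward to open and reversing to close.
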(event `/Game/InteractionSystem/BPI_Interactable.Interact`
  (params (Interactor :type "Actor Object Reference"))
  (if (`self.IsOpen?`)
    (`self.CloseDoor`)
    (else
      (`self.OpenDoor`))))

(event `OpenDoor`
  (set `self.IsOpen?` true)
  (`GameplayStatics.PlaySoundAtLocation` "/Engine/VREditor/Sounds/UI/Enter_Simulate.Enter_Simulate" (`self.K2_GetActorLocation`) (struct) 1.0 1.0 0.0 null null null null)
  (bind (_direction _z_rotation) (`Timeline|OpenDoorTimeline` :!label _label)
    (:`Update`
      (`SceneComponent.K2_SetRelativeRotation` (`self.Door`) (`KismetMathLibrary.MakeRotator` 0.0 0.0 _z_rotation) false false))))

(event `CloseDoor`
  (set `self.IsOpen?` false)
  (`GameplayStatics.PlaySoundAtLocation` "/Engine/VREditor/Sounds/UI/Leave_Simulate.Leave_Simulate" (`self.K2_GetActorLocation`) (struct) 1.0 1.0 0.0 null null null null)
  (goto _label :!via `Reverse`))

(fn `UserConstructionScript`)