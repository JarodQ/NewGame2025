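; Player component that lets a third-person character place, rotate and destroy building pieces loaded from DT_BuildParts.
; In build mode, Tick traces from the camera to move a preview mesh, then box-traces there to set CanBuild and the good or bad material.
; Enhanced Input spawns the selected Blueprint, rotates it on a looping timer, or destroys traced "Buildable" actors.
; Mouse wheel changes pieces, resetting a DoOnce so the preview is recreated.
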(event `self.ReceiveBeginPlay`
  (bind _asbp_third_person_character (cast `/Game/ThirdPerson/Blueprints/BP_ThirdPersonCharacter` (`self.GetOwner`)))
  (set `self.Player BP` _asbp_third_person_character)
  (set `self.Camera` (`/Game/ThirdPerson/Blueprints/BP_ThirdPersonCharacter.FollowCamera` _asbp_third_person_character))
  (bind _outrownames (`DataTableFunctionLibrary.GetDataTableRowNames` "/Game/BuildingSystem/DT_BuildParts.DT_BuildParts"))
  (for _array_element _outrownames
    (bind _returnvalue (`|GetDataTableRow` "/Game/BuildingSystem/DT_BuildParts.DT_BuildParts" _array_element)
      (:`then`
        (`KismetArrayLibrary.Array_Add` (`self.DT_buildables`) _returnvalue)))))

(event `self.ReceiveTick`
  (params (DeltaSeconds :type "Float (single-precision)"))
  (if (`self.inBuildMode`)
    (`self.PreviewLoop`)))

(event `PreviewLoop`
  (bind _build_preview_transform_location (`KismetMathLibrary.BreakTransform` (`self.Build Preview Transform`)))
  (bind (_returnvalue_location _returnvalue_rotation) (`KismetMathLibrary.BreakTransform` (`SceneComponent.K2_GetComponentToWorld` (`self.Camera`))))
  (bind _returnvalue (+ _returnvalue_location (0.0 0.0 200.0)))
  (bind (_outhit _returnvalue_2) (`KismetSystemLibrary.LineTraceSingle` _returnvalue (+ (* (`KismetMathLibrary.GetForwardVector` _returnvalue_rotation) 2000.0) _returnvalue) "TraceTypeQuery1"))
  (if _returnvalue_2
    (`|ExecutionSequence`
      (:`then_0`
        (`/Engine/EditorBlueprintResources/StandardMacros.DoOnce` false :!label _label
          (:`Completed`
            (bind _returnvalue_3 (`|AddComponentByClass` (`self.Player BP`) "/Script/Engine.StaticMeshComponent" false (`self.Build Preview Transform`)))
            (bind _output_get (set `self.Preview Mesh` _returnvalue_3))
            (`StaticMeshComponent.SetStaticMesh` _output_get (`.Mesh_5_7A827D7446BEDA96BFCA7C9ACF3B3B5A` (break `/Game/BuildingSystem/S_BuildParts` (`|GetArrayItem` (`self.DT_buildables`) (`self.buildableIndex`)))))
            (`PrimitiveComponent.SetCollisionEnabled` (`self.Preview Mesh`) "QueryOnly"))))
      (:`then_1`
        (bind _output_get_2 (set `self.Build Preview Transform` (`KismetMathLibrary.MakeTransform` (`.Location` (`GameplayStatics.BreakHitResult` _outhit)) (`self.Build Preview Rotation`))))
        (`SceneComponent.K2_SetWorldTransform` (`self.Preview Mesh`) _output_get_2 false false)
        (bind (_outhit_2 _returnvalue_4) (`KismetSystemLibrary.BoxTraceSingleForObjects` :`Start` _build_preview_transform_location :`End` _build_preview_transform_location :`HalfSize` (`.CollisionSize_14_18ADC1384916523277E0D6BA6F929EDC` (break `/Game/BuildingSystem/S_BuildParts` (`|GetArrayItem` (`self.DT_buildables`) (`self.buildableIndex`)))) :`ObjectTypes` (`|MakeArray` "ObjectTypeQuery7" :!type "EObjectTypeQuery Enum") :`DrawDebugType` "ForOneFrame"))
        (set `self.canBuild` (not _returnvalue_4))
        (`PrimitiveComponent.SetMaterial` (`self.Preview Mesh`) 0 (select `bool` _returnvalue_4 :`false` "/Game/BuildingSystem/M_BuildingPreview_Good.M_BuildingPreview_Good" :`true` "/Game/BuildingSystem/M_BuildingPreview_Bad.M_BuildingPreview_Bad" :!type "MaterialInterface Object Reference"))))))

(event `ResetBuildMode`
  (goto _label :!via `Reset`))

(event `EnhancedInput|/Game/ThirdPerson/Input/Actions/IA_Build`
  (params (ActionValue :type Boolean) (ElapsedSeconds :type "Float (double-precision)") (TriggeredSeconds :type "Float (double-precision)") (InputAction :type "InputAction Object Reference" :default "/Game/ThirdPerson/Input/Actions/IA_Build.IA_Build"))
  (:`Started`
    (if (not (`self.inBuildMode`))
      (set `self.inBuildMode` true)
      (else
        (set `self.inBuildMode` false :!label _label_2)
        (bind _preview_mesh (`self.Preview Mesh`)
          (:`then`
            (`StaticMeshComponent.SetStaticMesh` _preview_mesh null)
            (set `self.Preview Mesh` null)
            (`self.ResetBuildMode`))
          (:`else`))))))

(event `StopBuildMode`
  (goto _label_2))

(event `EnhancedInput|/Game/ThirdPerson/Input/Actions/IA_PlaceBuild`
  (params (ActionValue :type Boolean) (ElapsedSeconds :type "Float (double-precision)") (TriggeredSeconds :type "Float (double-precision)") (InputAction :type "InputAction Object Reference" :default "/Game/ThirdPerson/Input/Actions/IA_PlaceBuild.IA_PlaceBuild"))
  (:`Started`
    (if (and (`self.inBuildMode`) (`self.canBuild`))
      (`|SpawnActorFromClass` (`.Blueprint_8_9E37D7CA42B944A1533EA499927CCE04` (break `/Game/BuildingSystem/S_BuildParts` (`|GetArrayItem` (`self.DT_buildables`) (`self.buildableIndex`)))) (`self.Build Preview Transform`) "AlwaysSpawn" "MultiplyWithRoot" null null)
      (if (`self.buildOnce`)
        (`self.StopBuildMode`)))))

(event `EnhancedInput|/Game/ThirdPerson/Input/Actions/IA_RotateBuild`
  (params (ActionValue :type Boolean) (ElapsedSeconds :type "Float (double-precision)") (TriggeredSeconds :type "Float (double-precision)") (InputAction :type "InputAction Object Reference" :default "/Game/ThirdPerson/Input/Actions/IA_RotateBuild.IA_RotateBuild"))
  (:`Triggered`
    (`KismetSystemLibrary.K2_ClearAndInvalidateTimerHandle` (`self.Rotate Build Preview Loop`) :!label _label_3)
    (set `self.Rotate Build Preview Loop` (struct)))
  (:`Started`
    (bind _returnvalue (`KismetSystemLibrary.K2_SetTimerDelegate` (delegate `Rotate Preview`) 0.05 true))
    (set `self.Rotate Build Preview Loop` _returnvalue))
  (:`Canceled`
    (goto _label_3))
  (:`Completed`
    (goto _label_3)))

(event `Rotate Preview`
  (bind (_build_preview_transform_location _build_preview_transform_rotation) (`KismetMathLibrary.BreakTransform` (`self.Build Preview Transform`)))
  (set `self.Build Preview Rotation` (`KismetMathLibrary.ComposeRotators` _build_preview_transform_rotation (struct :`Yaw` 5.0))))

(event `Key|MouseScrollUp`
  (params (Key :type "Key Structure"))
  (:`Pressed`
    (set `self.buildableIndex` (`KismetMathLibrary.Clamp` (+ (`self.buildableIndex`) 1) 0 (- (`KismetArrayLibrary.Array_Length` (`self.DT_buildables`)) 1)))
    (bind _preview_mesh (`self.Preview Mesh` :!label _label_4)
      (:`then`
        (`StaticMeshComponent.SetStaticMesh` _preview_mesh null)
        (set `self.Preview Mesh` null)
        (`self.ResetBuildMode`))
      (:`else`))))

(event `Key|MouseScrollDown`
  (params (Key :type "Key Structure"))
  (:`Pressed`
    (set `self.buildableIndex` (`KismetMathLibrary.Clamp` 0 (- (`self.buildableIndex`) 1) (- (`KismetArrayLibrary.Array_Length` (`self.DT_buildables`)) 1)))
    (goto _label_4)))

(event `EnhancedInput|/Game/ThirdPerson/Input/Actions/IA_Destroy`
  (params (ActionValue :type Boolean) (ElapsedSeconds :type "Float (double-precision)") (TriggeredSeconds :type "Float (double-precision)") (InputAction :type "InputAction Object Reference" :default "/Game/ThirdPerson/Input/Actions/IA_Destroy.IA_Destroy"))
  (bind (_returnvalue_location _returnvalue_rotation) (`KismetMathLibrary.BreakTransform` (`SceneComponent.K2_GetComponentToWorld` (`self.Camera`))))
  (bind _returnvalue (+ _returnvalue_location (0.0 0.0 200.0)))
  (:`Started`
    (bind (_outhit _returnvalue_2) (`KismetSystemLibrary.LineTraceSingle` _returnvalue (+ (* (`KismetMathLibrary.GetForwardVector` _returnvalue_rotation) 2000.0) _returnvalue) "TraceTypeQuery1"))
    (if _returnvalue_2
      (bind (_bblockinghit _binitialoverlap _time _distance _location _impactpoint _normal _impactnormal _physmat _hitactor) (`GameplayStatics.BreakHitResult` _outhit))
      (if (`Actor.ActorHasTag` _hitactor "Buildable")
        (`Actor.K2_DestroyActor` _hitactor)))))