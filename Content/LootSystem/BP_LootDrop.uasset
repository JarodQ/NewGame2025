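; BP_LootDrop is a world loot item that disappears when a BP_ThirdPersonCharacter overlaps it.
; The construction script uses the DropTable row handle in ItemData to set the static mesh from a data table and resets actor scale.
; After a short delay on BeginPlay, it adds a scaled sphere component and enables pickup.
; Overlap only destroys the actor, with no item granted here.
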(event `self.ReceiveBeginPlay`
  (`KismetSystemLibrary.Delay` 2.0)
  (`AddComponent|NODE_AddSphereComponent-1` :`RelativeTransform` (`KismetMathLibrary.MakeTransform` (0.0 0.0 0.0) (struct) (1.75 1.75 1.75)))
  (set `self.CanPickUp?` true))

(event `self.ReceiveActorBeginOverlap`
  (params (OtherActor :type "Actor Object Reference"))
  (if (`self.CanPickUp?`)
    (cast `/Game/ThirdPerson/Blueprints/BP_ThirdPersonCharacter` OtherActor)
    (`self.K2_DestroyActor`)))

(fn `UserConstructionScript`
  (bind _itemdata (`self.itemData`))
  (bind _returnvalue (`|GetDataTableRow` (break `DataTableRowHandle` (break `/Game/LootSystem/S_DropTable` _itemdata)) (`.RowName` (break `DataTableRowHandle` (break `/Game/LootSystem/S_DropTable` _itemdata))))
    (:`then`
      (`StaticMeshComponent.SetStaticMesh` (`self.StaticMesh`) (`.StaticMesh_9_7F4561A34C1F2E9AD596F1A4E1A0CA24` (break `/Game/LootSystem/S_Drops` _returnvalue)))
      (`self.SetActorScale3D` (1.0 1.0 1.0)))))